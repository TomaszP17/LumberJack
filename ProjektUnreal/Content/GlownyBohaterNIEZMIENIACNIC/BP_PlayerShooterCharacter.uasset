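; Player shooter character Blueprint that handles opening and closing the pause menu.
; The Pause key calls PauseGame, which creates and caches the menu widget if needed, adds it to the viewport and switches to UI-only input with a visible cursor.
; UnPausedGame removes all widgets and restores game-only input with a hidden cursor.
; Both functions call SetGamePaused with false, so the game keeps running behind the menu.
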(event EventBeginPlay
  (|CallParentFunction) ; This node is disabled and will not be called.\nDrag off pins to build functionality.
)

(event Collision|EventActorBeginOverlap
  (params (OtherActor :type Actor%20Object%20Reference))
  (|CallParentFunction OtherActor) ; This node is disabled and will not be called.\nDrag off pins to build functionality.
)

(event EventTick
  (params (DeltaSeconds :type Float%20%28single-precision%29))
  (|CallParentFunction DeltaSeconds) ; This node is disabled and will not be called.\nDrag off pins to build functionality.
)

(event Input|KeyboardEvents|Pause
  (params (Key :type Key%20Structure :default "None"))
  (:Pressed
    (CallFunction|PauseGame)))

(fn ConstructionScript
  (|CallParentFunction))

(fn PauseGame
  (Game|SetGamePaused false)
  (Utilities|IsValid (Variables|Default|GetPauseMenu)
    (:Is%20Valid
      _)
    (:Is%20Not%20Valid
      (bind _returnvalue (UserInterface|CreateWidget "/Game/PauseMenu/PauseMenuWidget.PauseMenuWidget_C" (Game|GetPlayerController 0)))
      (Variables|Default|SetPauseMenu _returnvalue)))
  (UserInterface|Viewport|AddtoViewport (Variables|Default|GetPauseMenu) 0)
  (Input|SetInputModeUIOnly (Game|GetPlayerController 0) (Variables|Default|GetPauseMenu) "DoNotLock")
  (Variables|/Script/Engine.PlayerController|SetbShowMouseCursor (Game|GetPlayerController 0) true))

(fn UnPausedGame
  (bind _returnvalue (Game|GetPlayerController 0))
  (Game|SetGamePaused false)
  (Viewport|RemoveAllWidgets)
  (Input|SetInputModeGameOnly _returnvalue)
  (Variables|/Script/Engine.PlayerController|SetbShowMouseCursor _returnvalue false))
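; Enemy turret Blueprint that tracks the player pawn and continuously fires projectiles at it, with no range or line-of-sight check.
; Tick drives UpdateRotation, which eases TurretGun toward the player via RInterpTo, with pitch offset by BarrelLength and clamped.
; Tick also calls FireWeapons, where a Delay throttles spawning of BP_PociskWiezyczki at the Barrel socket to once per FireInterval.
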(event Custom|Update%20Rotation
  (bind _returnvalue (Game|Player|GetPlayerPawn 0))
  (bind _turretgun (Variables|Default|GetTurretGun))
  (bind _returnvalue_2 (Transformation|GetWorldLocation _turretgun))
  (bind _returnvalue_3 (Transformation|GetActorLocation _returnvalue))
  (bind _returnvalue_4 (Math|Rotator|FindLookatRotation _returnvalue_2 _returnvalue_3))
  (bind (_roll _pitch _yaw) (Math|Rotator|BreakRotator _returnvalue_4))
  ;[1 1 1] Obracanie wiezyczki
  (Transformation|SetWorldRotation (Variables|Default|GetTurretGun) (Math|Interpolation|RInterpTo (Transformation|GetWorldRotation (Variables|Default|GetTurretGun)) (Math|Rotator|MakeRotator 0.0 (Math|Float|ClampAngle (+ _pitch (Variables|TurretSettings|GetBarrelLength)) -1e+01 35.0) _yaw) (Variables|Default|GetDeltaTime) (Variables|TurretSettings|GetRotationSpeed)) false false))

(event Custom|Fire%20Weapons
  ;[1 1 1] Strzelanie
  (Utilities|FlowControl|Delay (Variables|TurretSettings|GetFireInterval))
  (Game|SpawnActorfromClass "/Game/ToonTanks/Assets/Meshes/BP_PociskWiezyczki.BP_PociskWiezyczki_C" (Transformation|GetSocketTransform (Variables|Default|GetTurretGun) "Barrel" "RTS_World") "Undefined" 0 0))

(event EventBeginPlay)

(event Collision|EventActorBeginOverlap
  (params (OtherActor :type Actor%20Object%20Reference)))

(event EventTick
  (params (DeltaSeconds :type Float%20%28single-precision%29))
  ;[1 1 1] Game Loop
  (Variables|Default|SetDeltaTime DeltaSeconds)
  (CallFunction|UpdateRotation)
  (CallFunction|FireWeapons))

(fn ConstructionScript)